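; BP_MainHubPortal is a main hub portal actor whose only scripted behavior is keeping its audio volume in line with game settings.
; On BeginPlay it caches the Game_GameInstance and applies the saved SFX volume to its Audio component.
; It then binds to the game instance's music volume change event, not an SFX one, so later music volume changes overwrite that multiplier.
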(event `self.ReceiveBeginPlay`
  (bind _asgame_game_instance (cast `Game_GameInstance` (`GameplayStatics.GetGameInstance`)))
  (bind _output_get (set `self.GameInstance` _asgame_game_instance))
  (bind _returnvalue (`Game_GameInstance.GetSFXVolume` _output_get))
  (`AudioComponent.SetVolumeMultiplier` (`self.Audio`) _returnvalue)
  (add `Game_GameInstance.OnMusicVolumeChanged` (`self.GameInstance`) (delegate `HandleVolumeChanged`)))

(event `HandleVolumeChanged`
  (params (a_newVolume :type "Float (single-precision)"))
  (`AudioComponent.SetVolumeMultiplier` (`self.Audio`) a_newVolume))

(fn `UserConstructionScript`)